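; BP_BasePlayerCharacter is a base player character Blueprint that turns raw keyboard input into state flags.
; Q, Left Shift, R and E set pressed flags that clear on release, and E also toggles an Eon flag.
; Z latches its flag for a fixed delay, ignoring repeat presses meanwhile.
; Tab flip-flops global time dilation between slow motion and normal speed.
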(event EventBeginPlay)

(event Collision|EventActorBeginOverlap
  (params (OtherActor :type Actor%20Object%20Reference)))

(event EventTick
  (params (DeltaSeconds :type Float%20%28single-precision%29)))

(event Input|KeyboardEvents|Tab
  (params (Key :type Key%20Structure :default "None"))
  (:Pressed
    (Utilities|FlowControl|FlipFlop
      (:A
        (Utilities|Time|SetGlobalTimeDilation 0.25))
      (:B
        (Utilities|Time|SetGlobalTimeDilation 1.0)))))

(event Input|KeyboardEvents|Z
  (params (Key :type Key%20Structure :default "None"))
  (:Pressed
    (if (not (Variables|Default|GetIsZPressed))
      (Variables|Default|SetIsZPressed true)
      (Utilities|FlowControl|Delay 2.7)
      (Variables|Default|SetIsZPressed false))))

(event Input|KeyboardEvents|Q
  (params (Key :type Key%20Structure :default "None"))
  (:Pressed
    (Variables|Default|SetIsQPressed true))
  (:Released
    (Variables|Default|SetIsQPressed false)))

(event Input|KeyboardEvents|E
  (params (Key :type Key%20Structure :default "None"))
  (:Pressed
    (if (Variables|Default|GetEon)
      (Variables|Default|SetEon false)
      (Variables|Default|SetIsEPressed true)
      (else
        (Variables|Default|SetEon true)
        (Variables|Default|SetIsEPressed true))))
  (:Released
    (Variables|Default|SetIsEPressed false)))

(event Input|KeyboardEvents|R
  (params (Key :type Key%20Structure :default "None"))
  (:Pressed
    (Variables|Default|SetIsRPressed true))
  (:Released
    (Variables|Default|SetIsRPressed false)))

(event Input|KeyboardEvents|LeftShift
  (params (Key :type Key%20Structure :default "None"))
  (:Pressed
    (Variables|Default|SetIsLShiftPressed true))
  (:Released
    (Variables|Default|SetIsLShiftPressed false)))

(fn ConstructionScript)
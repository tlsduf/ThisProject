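; Base enemy character that manages an overhead HP bar widget and spawns a Bp_asdf actor at its Cube component's location on BeginPlay.
; BeginPlay also sets itself as the HP bar widget's owner.
; Taking damage reveals the bar, and a retriggerable delay hides it after a period without further hits.
; Tick keeps the bar hidden once the enemy is dead; a damage-widget hookup is left unconnected.
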(event EventBeginPlay
  (Utilities|FlowControl|Sequence
    (:then_0
      (bind _aswbp_hpbar (Utilities|Casting|CastToWBP_HPBar (UserInterface|GetUserWidgetObject (Variables|Default|GetHPBar))))
      (Variables|/Game/MyCharacter/UI/WBP_HPBar.WBP_HPBar_C|SetOwnActor _aswbp_hpbar self))
    (:then_2
      (Game|SpawnActorfromClass "/Game/MyCharacter/UI/bp_asdf.bp_asdf_C" (Math|Conversions|ToTransform(Vector) (Transformation|GetWorldLocation (Variables|Default|GetCube))) "Undefined" 0 0))))

(event Collision|EventActorBeginOverlap
  (params (OtherActor :type Actor%20Object%20Reference)))

(event EventTick
  (params (DeltaSeconds :type Float%20%28single-precision%29))
  (Utilities|FlowControl|Sequence
    (:then_0
      (if (Class|MyRoguelikeCharacter|IsDead)
        (Development|SetHiddeninGame (Variables|Default|GetHPBar) true false)))))

(event Game|Damage|EventAnyDamage
  (params (Damage :type Float%20%28single-precision%29) (DamageType :type Damage%20Type%20Object%20Reference) (InstigatedBy :type Controller%20Object%20Reference) (DamageCauser :type Actor%20Object%20Reference))
  (Utilities|FlowControl|Sequence
    (:then_0
      (Development|SetHiddeninGame (Variables|Default|GetHPBar) false false)
      (Utilities|FlowControl|RetriggerableDelay 1e+01)
      (Development|SetHiddeninGame (Variables|Default|GetHPBar) true false))))

(fn ConstructionScript)
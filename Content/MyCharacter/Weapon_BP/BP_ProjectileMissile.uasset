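; BP_ProjectileMissile is a projectile actor that homes on actors tagged "Enemy" and destroys itself after a fixed delay.
; Every tick it checks all tagged actors against ClosestDistance, switching ProjectileMovementComponent homing on or off for each.
; ClosestDistance is never updated, so the last actor checked decides whether homing stays on, rather than the nearest.
; Tick also draws a fixed-radius debug sphere around the missile.
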(event EventBeginPlay
  (Utilities|FlowControl|Sequence
    (:then_0
      (Utilities|FlowControl|Delay 2e+01)
      (Actor|DestroyActor))))

(event Collision|EventActorBeginOverlap
  (params (OtherActor :type Actor%20Object%20Reference)))

(event EventTick
  (params (DeltaSeconds :type Float%20%28single-precision%29))
  (bind _projectilemovementcomponent (Variables|Default|GetProjectileMovementComponent))
  (Utilities|FlowControl|Sequence
    (:then_0
      (bind _outactors (Actor|GetAllActorswithTag "Enemy"))
      (for _array_element _outactors
        (if (< (Math|Vector|Distance(Vector) (Transformation|GetActorLocation) (Transformation|GetWorldLocation (Variables|/Script/Engine.Actor|GetRootComponent _array_element))) (Variables|Default|GetClosestDistance))
          (Variables|/Script/Engine.ProjectileMovementComponent|SetbIsHomingProjectile _projectilemovementcomponent true)
          (Variables|/Script/Engine.ProjectileMovementComponent|SetHomingTargetComponent _projectilemovementcomponent (Variables|/Script/Engine.Actor|GetRootComponent _array_element))
          (else
            (Variables|/Script/Engine.ProjectileMovementComponent|SetbIsHomingProjectile _projectilemovementcomponent false)))))
    (:then_1
      (if true
        (Rendering|Debug|DrawDebugSphere (Transformation|GetActorLocation) 1e+03 12 "(R=1.000000,G=0.030093,B=0.010197,A=1.000000)" 0.0)
        (else
          (Rendering|Debug|DrawDebugSphere (Transformation|GetActorLocation) 1e+03 12 "(R=1.000000,G=1.000000,B=1.000000,A=1.000000)" 0.0))))))

(fn ConstructionScript)
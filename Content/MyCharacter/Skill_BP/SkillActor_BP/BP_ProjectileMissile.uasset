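; BP_ProjectileMissile is a skill missile actor that, in its active graph, only destroys itself ten seconds after spawning.
; A disconnected, never-executed branch holds homing logic that loops over actors tagged Enemy and compares their distance to ClosestDistance.
; That branch toggles homing on the ProjectileMovementComponent per enemy without updating the threshold, so later enemies override earlier results.
; Overlap, Tick and the construction script are empty.
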(event EventBeginPlay
  (Utilities|FlowControl|Sequence
    (:then_0
      (Utilities|FlowControl|Delay 1e+01)
      (Actor|DestroyActor))))

(event Collision|EventActorBeginOverlap
  (params (OtherActor :type Actor%20Object%20Reference)))

(event EventTick
  (params (DeltaSeconds :type Float%20%28single-precision%29)))

(fn ConstructionScript)